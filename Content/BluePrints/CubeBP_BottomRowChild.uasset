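; Bottom-row child cube that hatches a purple ball into a coil snake when the ball lands on it.
; On overlap it runs the parent cube's logic, then continues only for BallBP_PurpleChild actors.
; After a delay it hides the ball, spawns a scaled CoilSnakeBP above it with a cone mesh, then destroys the ball.
; Short delays sequence the swap.
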(event `self.ReceiveActorBeginOverlap`
  (params (OtherActor :type "Actor Object Reference"))
  (`parent.ReceiveActorBeginOverlap` OtherActor)
  (bind _asball_bp_purple_child (cast `/Game/BluePrints/BallBP_PurpleChild` OtherActor))
  (`KismetSystemLibrary.Delay` 1.0)
  (`SceneComponent.SetVisibility` (`/Game/BluePrints/BallBP.Sphere` _asball_bp_purple_child) false false)
  (`KismetSystemLibrary.Delay` 0.01)
  (bind _returnvalue (`|SpawnActorFromClass` "/Game/BluePrints/CoilSnakeBP.CoilSnakeBP_C" (`KismetMathLibrary.MakeTransform` (`KismetMathLibrary.TransformLocation` (`self.GetTransform` _asball_bp_purple_child) (0.0 0.0 200.0)) (struct) (0.3 0.3 0.5)) "Undefined" "OverrideRootScale"))
  (`StaticMeshComponent.SetStaticMesh` (`/Game/BluePrints/BallBP.Sphere` _returnvalue) "/Game/Assets/Shape_Cone.Shape_Cone")
  (`KismetSystemLibrary.Delay` 0.1)
  (`self.K2_DestroyActor` _asball_bp_purple_child))

(fn `UserConstructionScript`
  (`parent.UserConstructionScript`))