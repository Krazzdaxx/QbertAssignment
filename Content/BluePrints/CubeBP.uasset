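; Cube tile for a Q*bert-style game that lights up and scores when the player lands on it.
; On first overlap by QBert_Blueprint, it switches to the pulse material, marks itself colored and increments the GameManager score.
; When the score reaches 28, it plays a sound and flashes every CubeBP between plain and pulse materials through nested ForEach loops with short Delays.
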(event `self.ReceiveActorBeginOverlap`
  (params (OtherActor :type "Actor Object Reference"))
  (cast `/Game/BluePrints/QBert_Blueprint` OtherActor)
  (bind _asgame_manager (cast `/Game/BluePrints/GameManager` (`GameplayStatics.GetGameState`)))
  (if (== (`self.BoxColor`) 0)
    (set `/Game/BluePrints/GameManager.Score` (+ (`/Game/BluePrints/GameManager.Score` _asgame_manager) 1) _asgame_manager)
    (`PrimitiveComponent.SetMaterial` (`self.StaticMeshComponent`) 0 "/Game/StarterContent/Materials/M_Tech_Hex_Tile_Pulse.M_Tech_Hex_Tile_Pulse")
    (set `self.BoxColor` 1)
    (bind _asgame_manager_2 (cast `/Game/BluePrints/GameManager` (`GameplayStatics.GetGameState`)))
    (if (== (`/Game/BluePrints/GameManager.Score` _asgame_manager_2) 28)
      (`GameplayStatics.PlaySound2D` "/Game/Audio/32_Cue.32_Cue")
      (bind _outactors (`GameplayStatics.GetAllActorsOfClass` "CubeBP_C"))
      (for _array_element _outactors
        (`PrimitiveComponent.SetMaterial` (`StaticMeshActor.StaticMeshComponent` _array_element) 0 "/Game/StarterContent/Materials/M_Tech_Hex_Tile.M_Tech_Hex_Tile" :!label _label)
        (`KismetSystemLibrary.Delay` 0.2)
        (for _array_element_2 _outactors
          (`PrimitiveComponent.SetMaterial` (`StaticMeshActor.StaticMeshComponent` _array_element_2) 0 "/Game/StarterContent/Materials/M_Tech_Hex_Tile_Pulse.M_Tech_Hex_Tile_Pulse" :!label _label_2)
          (`KismetSystemLibrary.Delay` 0.2)
          (for _array_element_3 _outactors
            (`PrimitiveComponent.SetMaterial` (`StaticMeshActor.StaticMeshComponent` _array_element_3) 0 "/Game/StarterContent/Materials/M_Tech_Hex_Tile.M_Tech_Hex_Tile" :!label _label_3)
            (`KismetSystemLibrary.Delay` 0.2)
            (for _array_element_4 _outactors
              (`PrimitiveComponent.SetMaterial` (`StaticMeshActor.StaticMeshComponent` _array_element_4) 0 "/Game/StarterContent/Materials/M_Tech_Hex_Tile_Pulse.M_Tech_Hex_Tile_Pulse")))
          (goto _label_3))
        (goto _label_2))
      (goto _label))))

(fn `UserConstructionScript`)