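; Green ball pickup Blueprint for a Q*bert game, extending a parent ball Blueprint.
; On overlap with Q*Bert it adds to the GameManager's green ball score bonus, plays a sound and sets GreenBallPaused.
; The sphere then hides and the actor destroys itself after a delay, without clearing the flag.
; Tick calls the parent, then reapplies the green material every frame while the flag is off.
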(event `self.ReceiveTick`
  (params (DeltaSeconds :type "Float (single-precision)"))
  (`parent.ReceiveTick` 0.0)
  (bind _asgame_manager (cast `/Game/BluePrints/GameManager` (`GameplayStatics.GetGameState`)))
  (if (not (`/Game/BluePrints/GameManager.GreenBallPaused` _asgame_manager))
    (`PrimitiveComponent.SetMaterial` (`self.Sphere`) 0 "/Game/StarterContent/Materials/GreenBall.GreenBall")))

(event `self.ReceiveActorBeginOverlap`
  (params (OtherActor :type "Actor Object Reference"))
  (cast `/Game/BluePrints/QBert_Blueprint` OtherActor)
  (bind _asgame_manager (cast `/Game/BluePrints/GameManager` (`GameplayStatics.GetGameState`)))
  (set `/Game/BluePrints/GameManager.GreenBallScoreBonus` (+ (`/Game/BluePrints/GameManager.GreenBallScoreBonus` _asgame_manager) 100) _asgame_manager)
  (`GameplayStatics.PlaySound2D` "/Game/Audio/Extra_Bert_Cue.Extra_Bert_Cue")
  (bind _asgame_manager_2 (cast `/Game/BluePrints/GameManager` (`GameplayStatics.GetGameState`)))
  (set `/Game/BluePrints/GameManager.GreenBallPaused` true _asgame_manager_2)
  (`SceneComponent.SetVisibility` (`self.Sphere`) false false)
  (`KismetSystemLibrary.Delay` 5.0)
  (`self.K2_DestroyActor`))

(fn `UserConstructionScript`
  (`parent.UserConstructionScript`))