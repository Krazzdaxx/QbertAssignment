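; GameManager handles the pause menu and a timed pause flag for the green ball.
; The Pause Game input creates the PauseMenu widget if none is valid, switches to UI-only input, adds it to the viewport and pauses the game.
; Tick watches GreenBallPaused and clears it after a five-second Delay.
; The InreaseScore function and construction script are empty.
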(event `self.ReceiveTick`
  (params (DeltaSeconds :type "Float (single-precision)"))
  (if (`self.GreenBallPaused`)
    (`KismetSystemLibrary.Delay` 5.0)
    (set `self.GreenBallPaused` false)))

(event `InputAction|Pause Game`
  (params (Key :type "Key Structure" :default "AnyKey"))
  (bind _pause_menu_ref (`self.Pause Menu Ref`))
  (:`Pressed`
    (`/Engine/EditorBlueprintResources/StandardMacros.IsValid` (`self.Pause Menu Ref`)
      (:`Is Valid`
        _)
      (:`Is Not Valid`
        (bind _returnvalue (`|CreateWidget` "/Game/BluePrints/PauseMenu.PauseMenu_C"))
        (set `self.Pause Menu Ref` _returnvalue)))
    (`WidgetBlueprintLibrary.SetInputMode_UIOnlyEx` (`GameplayStatics.GetPlayerController` 0) _pause_menu_ref)
    (`UserWidget.AddToViewport` _pause_menu_ref 0)
    (`GameplayStatics.SetGamePaused` true)))

(fn `InreaseScore`)

(fn `UserConstructionScript`)