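; BallBP is a ball actor that descends in random diagonal steps and can be paused through the GameManager's GreenBallPaused flag.
; Tick reads that flag from the game state and applies the PausedColor material while it is set, with no branch restoring the original.
; Otherwise a Delay on Tick paces movement to roughly two-second intervals, rechecks the flag, then offsets the ball down and along either X or Y without sweep.
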(event `self.ReceiveTick`
  (params (DeltaSeconds :type "Float (single-precision)"))
  (bind _asgame_manager (cast `/Game/BluePrints/GameManager` (`GameplayStatics.GetGameState`)))
  (bind _greenballpaused (`/Game/BluePrints/GameManager.GreenBallPaused` _asgame_manager))
  (if _greenballpaused
    (`PrimitiveComponent.SetMaterial` (`self.Sphere`) 0 "/Game/StarterContent/Materials/PausedColor.PausedColor")
    (else
      (`KismetSystemLibrary.Delay` 2.0)
      (if _greenballpaused
        _
        (elif (== (`KismetMathLibrary.RandomIntegerInRange` 0 1) 0)
          (`self.K2_AddActorWorldOffset` (50.0 0.0 -50.0))
          (else
            (`self.K2_AddActorWorldOffset` (0.0 50.0 -50.0))))))))

(fn `UserConstructionScript`)