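; Coil Snake enemy actor that chases the player pawn in stepped hops, changing height with each move.
; Tick reads GreenBallPaused from the GameManager game state and swaps the sphere to a paused material while set.
; Otherwise a one-second Delay on Tick paces each hop, which follows the axis of greater X or Y distance to the player.
; Hops are fixed unswept offsets, climbing toward negative X or Y and descending toward positive.
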(event `self.ReceiveTick`
  (params (DeltaSeconds :type "Float (single-precision)"))
  (bind _returnvalue (`GameplayStatics.GetPlayerPawn` 0))
  (bind _asgame_manager (cast `/Game/BluePrints/GameManager` (`GameplayStatics.GetGameState`)))
  (bind _greenballpaused (`/Game/BluePrints/GameManager.GreenBallPaused` _asgame_manager))
  (if _greenballpaused
    (`PrimitiveComponent.SetMaterial` (`self.Sphere`) 0 "/Game/StarterContent/Materials/PausedColor.PausedColor")
    (else
      (`PrimitiveComponent.SetMaterial` (`self.Sphere`) 0 "/Game/StarterContent/Materials/CoilSnake.CoilSnake")
      (`KismetSystemLibrary.Delay` 1.0)
      (if _greenballpaused
        _
        (elif (> (`KismetMathLibrary.VSize` (- (`KismetMathLibrary.Conv_DoubleToVector` (.x (`self.K2_GetActorLocation`))) (`KismetMathLibrary.Conv_DoubleToVector` (.x (`self.K2_GetActorLocation` _returnvalue))))) (`KismetMathLibrary.VSize` (- (`KismetMathLibrary.Conv_DoubleToVector` (.y (`self.K2_GetActorLocation`))) (`KismetMathLibrary.Conv_DoubleToVector` (.y (`self.K2_GetActorLocation` _returnvalue))))))
          (if (> (.x (`self.K2_GetActorLocation`)) (.x (`self.K2_GetActorLocation` (`GameplayStatics.GetPlayerPawn` 0))))
            (`self.K2_AddActorWorldOffset` (-50.0 0.0 50.0))
            (else
              (`self.K2_AddActorWorldOffset` (50.0 0.0 -50.0))))
          (elif (> (.y (`self.K2_GetActorLocation`)) (.y (`self.K2_GetActorLocation` (`GameplayStatics.GetPlayerPawn` 0))))
            (`self.K2_AddActorWorldOffset` (0.0 -50.0 50.0))
            (else
              (`self.K2_AddActorWorldOffset` (0.0 50.0 -50.0)))))))))

(fn `UserConstructionScript`)