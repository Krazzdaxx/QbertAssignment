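; Red ball hazard for a Q*bert game, apparently a child of BallBP, that kills Q*bert on contact.
; Tick runs the parent logic, then applies the red material whenever the GameManager's GreenBallPaused flag is off.
; Overlapping Q*bert shows the curse text and plays a sound, then after a short delay calls QbertDied on the player pawn and destroys all BallBP actors.
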(event `self.ReceiveTick`
  (params (DeltaSeconds :type "Float (single-precision)"))
  (`parent.ReceiveTick` 0.0)
  (bind _asgame_manager (cast `/Game/BluePrints/GameManager` (`GameplayStatics.GetGameState`)))
  (if (not (`/Game/BluePrints/GameManager.GreenBallPaused` _asgame_manager))
    (`PrimitiveComponent.SetMaterial` (`self.Sphere`) 0 "/Game/StarterContent/Materials/RedBall.RedBall")))

(event `self.ReceiveActorBeginOverlap`
  (params (OtherActor :type "Actor Object Reference"))
  (bind _asqbert_blueprint (cast `/Game/BluePrints/QBert_Blueprint` OtherActor))
  (set `/Game/BluePrints/QBert_Blueprint.CurseTextVisibility` true _asqbert_blueprint)
  (`GameplayStatics.PlaySound2D` "/Game/Audio/Sware1_Cue.Sware1_Cue")
  (`KismetSystemLibrary.Delay` 0.2)
  (bind _asqbert_blueprint_2 (cast `/Game/BluePrints/QBert_Blueprint` (`GameplayStatics.GetPlayerPawn` 0)))
  (`/Game/BluePrints/QBert_Blueprint.QbertDied` _asqbert_blueprint_2)
  (bind _outactors (`GameplayStatics.GetAllActorsOfClass` "/Game/BluePrints/BallBP.BallBP_C"))
  (for _array_element _outactors
    (`self.K2_DestroyActor` _array_element :!label _label))
  (goto _label))

(fn `UserConstructionScript`
  (`parent.UserConstructionScript`))