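; Player-controlled Q*bert that hops diagonally in fixed steps, with sound and a curse text display.
; Four input actions offset the actor instantly without sweep, then share a half-second input lockout to space out hops.
; Tick shows the TextRender while CurseTextVisibility is set, clearing the flag after a two-second delay.
; Helper functions decrement Lives on the GameManager game state at death and toggle input on the player pawn.
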(event `self.ReceiveTick`
  (params (DeltaSeconds :type "Float (single-precision)"))
  (if (`self.CurseTextVisibility`)
    (`SceneComponent.SetVisibility` (`self.TextRender`) true false)
    (`KismetSystemLibrary.Delay` 2.0)
    (set `self.CurseTextVisibility` false)
    (else
      (`SceneComponent.SetVisibility` (`self.TextRender`) false false))))

(event `InputAction|MoveUpAndRight`
  (params (Key :type "Key Structure" :default "AnyKey"))
  (:`Pressed`
    (`GameplayStatics.PlaySound2D` "/Game/Audio/Hop_Cue.Hop_Cue" 0.25 1.0)
    (`self.K2_AddActorWorldOffset` (0.0 -50.0 50.0))
    (`self.DisableInput` null :!label _label)
    (`KismetSystemLibrary.Delay` 0.5)
    (`self.EnableInput` (`GameplayStatics.GetPlayerController` 0))))

(event `InputAction|MoveUpAndLeft`
  (params (Key :type "Key Structure" :default "AnyKey"))
  (:`Pressed`
    (`GameplayStatics.PlaySound2D` "/Game/Audio/Hop_Cue.Hop_Cue" 0.25 1.0)
    (`self.K2_AddActorWorldOffset` (-50.0 0.0 50.0))
    (goto _label)))

(event `InputAction|MoveDownAndLeft`
  (params (Key :type "Key Structure" :default "AnyKey"))
  (:`Pressed`
    (`GameplayStatics.PlaySound2D` "/Game/Audio/Hop_Cue.Hop_Cue" 0.25 1.0)
    (`self.K2_AddActorWorldOffset` (0.0 50.0 -50.0))
    (goto _label)))

(event `InputAction|MoveDownAndRigt`
  (params (Key :type "Key Structure" :default "AnyKey"))
  (:`Pressed`
    (`GameplayStatics.PlaySound2D` "/Game/Audio/Hop_Cue.Hop_Cue" 0.25 1.0)
    (`self.K2_AddActorWorldOffset` (50.0 0.0 -50.0))
    (goto _label)))

(event `self.ReceiveBeginPlay`
  (`SceneComponent.SetVisibility` (`self.TextRender`) false false)
  (`self.EnableInput` (`GameplayStatics.GetPlayerController` 0)))

(fn `DisableQbertInput`
  (`self.DisableInput` (`GameplayStatics.GetPlayerPawn` 0) (`GameplayStatics.GetPlayerController` 0)))

(fn `EnableQbertInput`
  (`self.EnableInput` (`GameplayStatics.GetPlayerPawn` 0) (`GameplayStatics.GetPlayerController` 0)))

(fn `QbertDied`
  (bind _asgame_manager (cast `/Game/BluePrints/GameManager` (`GameplayStatics.GetGameState`)))
  (`/Engine/EditorBlueprintResources/StandardMacros.DecrementInt` (`/Game/BluePrints/GameManager.Lives` _asgame_manager)))

(fn `UserConstructionScript`)